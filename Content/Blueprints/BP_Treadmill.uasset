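; Treadmill Blueprint that fakes endless travel by looping two floor pieces along a spline with randomized scenery.
; Each Tick advances a normalized loop timer at a rate set by the GameInstance slider value and a global play rate.
; The floors sit half a loop apart, placed with constant-velocity spline sampling.
; When either floor wraps, its prop and ground-detail meshes are re-rolled, with a DoOnce guarding the second floor's swap.
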(event `self.ReceiveTick`
  (params (DeltaSeconds :type "Float (single-precision)"))
  ;[1 1 1] Tick
  (bind _output_get (set `self.playRate` (/ (`/Game/Blueprints/BP_GameInstance.SliderValue` (cast `/Game/Blueprints/BP_GameInstance` (`GameplayStatics.GetGameInstance`) :!pure true)) 1500.0)))
  (set `self.DeltaTimeForTimer` (* _output_get DeltaSeconds (`self.globalPlayRate`)))
  (`self.SetTimers`)
  (`self.SetPosFloor1`)
  (`self.SetPosFloor2`))

(event `SetPosFloor1`
  (bind _returnvalue_location (`KismetMathLibrary.BreakTransform` (`SplineComponent.GetTransformAtTime` (`self.Spline`) (`self.currentLoopTimer1`) "World" true false)))
  ;[1 1 1] Comment
  (`SceneComponent.K2_SetWorldLocation` (`self.Floor1`) _returnvalue_location false false))

(event `SetTimers`
  ;[1 1 1] Set timer event
  (if (> (+ (`self.currentLoopTimer1`) (`self.DeltaTimeForTimer`)) 1.0)
    (set `self.currentLoopTimer1` 0.0)
    (set `self.currentLoopTimer2` 0.5)
    (`self.SetRandomObjectsFloor1`)
    (else
      (set `self.currentLoopTimer1` (+ (`self.currentLoopTimer1`) (`self.DeltaTimeForTimer`)))
      (if (> (+ (`self.currentLoopTimer1`) 0.5) 1.0)
        (set `self.currentLoopTimer2` (- (`self.currentLoopTimer1`) 0.5))
        (`/Engine/EditorBlueprintResources/StandardMacros.DoOnce` false :!label _label
          (:`Completed`
            (`self.SetRandomObjectsFloor2`)))
        (else
          (set `self.currentLoopTimer2` (+ (`self.currentLoopTimer1`) 0.5))
          (goto _label :!via `Reset`))))))

(event `SetPosFloor2`
  (bind _returnvalue_location (`KismetMathLibrary.BreakTransform` (`SplineComponent.GetTransformAtTime` (`self.Spline`) (`self.currentLoopTimer2`) "World" true false)))
  ;[1 1 1] Comment
  (`SceneComponent.K2_SetWorldLocation` (`self.Floor2`) _returnvalue_location false false))

(fn `GetRandomFloorObject`
  (returns (NewParam :type "StaticMesh Object Reference"))
  (return (select `int` (`KismetMathLibrary.RandomIntegerInRange` 0 3) :`0` "/Game/MarketPlaceContent/AdvancedVillagePack/Meshes/SM_Flower_Var01.SM_Flower_Var01" :`1` "/Game/MarketPlaceContent/AdvancedVillagePack/Meshes/SM_Flower_Var02.SM_Flower_Var02" :`2` "/Game/MarketPlaceContent/AdvancedVillagePack/Meshes/SM_StoneFlat_Var05.SM_StoneFlat_Var05" :`3` "/Game/MarketPlaceContent/AdvancedVillagePack/Meshes/SM_Stonepath_Var01.SM_Stonepath_Var01" :!type "StaticMesh Object Reference")))

(fn `GetRandomObject`
  (returns (NewParam :type "StaticMesh Object Reference"))
  (return (select `int` (`KismetMathLibrary.RandomIntegerInRange` 0 8) :`0` "/Game/MarketPlaceContent/AdvancedVillagePack/Meshes/SM_Stone_Big_Var01.SM_Stone_Big_Var01" :`1` "/Game/MarketPlaceContent/AdvancedVillagePack/Meshes/SM_StreetLight_LightsOn.SM_StreetLight_LightsOn" :`2` "/Game/MarketPlaceContent/AdvancedVillagePack/Meshes/SM_Fence_Var03.SM_Fence_Var03" :`3` "/Game/MarketPlaceContent/AdvancedVillagePack/Meshes/SM_GrassPatch_Var01.SM_GrassPatch_Var01" :`4` "/Game/MarketPlaceContent/AdvancedVillagePack/Meshes/SM_Barrel.SM_Barrel" :`5` "/Game/MarketPlaceContent/AdvancedVillagePack/Meshes/SM_Cauldron.SM_Cauldron" :`6` "/Game/MarketPlaceContent/AdvancedVillagePack/Meshes/SM_Tree_Var01.SM_Tree_Var01" :`7` "/Game/MarketPlaceContent/AdvancedVillagePack/Meshes/SM_Well.SM_Well" :`8` "/Game/MarketPlaceContent/AdvancedVillagePack/Meshes/SM_Cart_Var01.SM_Cart_Var01" :!type "StaticMesh Object Reference")))

(fn `SetRandomObjectsFloor1`
  (for _array_element (`|MakeArray` (`self.RandomObject1`) (`self.RandomObject2`) (`self.RandomObject3`))
    (bind _newparam (`self.GetRandomObject`))
    (`StaticMeshComponent.SetStaticMesh` _array_element _newparam))
  (for _array_element_2 (`|MakeArray` (`self.RandomFloorObject1`) (`self.RandomFloorObject2`) (`self.RandomFloorObject3`))
    (bind _newparam_2 (`self.GetRandomFloorObject`))
    (`StaticMeshComponent.SetStaticMesh` _array_element_2 _newparam_2)))

(fn `SetRandomObjectsFloor2`
  (for _array_element (`|MakeArray` (`self.RandomObject4`) (`self.RandomObject5`) (`self.RandomObject6`))
    (bind _newparam (`self.GetRandomObject`))
    (`StaticMeshComponent.SetStaticMesh` _array_element _newparam))
  (for _array_element_2 (`|MakeArray` (`self.RandomFloorObject4`) (`self.RandomFloorObject5`) (`self.RandomFloorObject6`))
    (bind _newparam_2 (`self.GetRandomFloorObject`))
    (`StaticMeshComponent.SetStaticMesh` _array_element_2 _newparam_2)))

(fn `UserConstructionScript`)