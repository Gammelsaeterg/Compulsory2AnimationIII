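; BP_BigScreen is a video screen that shows and plays the NinjaCartoon media while the game instance's SliderValue is above 1400.
; BeginPlay opens the source on the MediaPlayer, then pauses it and hides the BigScreen component.
; Tick polls the slider value, using two DoOnce gates that reset each other so play/show and pause/hide each fire once per threshold crossing.
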(event `self.ReceiveBeginPlay`
  (bind _bsuccess (`MediaPlayer.OpenSourceLatent` (`self.MediaPlayer`) "/Game/Media/NinjaCartoon.NinjaCartoon" (make `MediaPlayerOptions` (struct :`Caption` -1 :`Metadata` -1 :`Script` -1 :`Subtitle` -1 :`Text` -1))))
  (set `self.canPlayVideo` _bsuccess)
  (`self.SetPause`))

(event `SetPause`
  (`MediaPlayer.Pause` (`self.MediaPlayer`))
  (`SceneComponent.SetVisibility` (`self.BigScreen`) false false))

(event `StartBigScreen`
  (`MediaPlayer.Play` (`self.MediaPlayer`))
  (`SceneComponent.SetVisibility` (`self.BigScreen`) true false))

(event `self.ReceiveTick`
  (params (DeltaSeconds :type "Float (single-precision)"))
  (if (> (`/Game/Blueprints/BP_GameInstance.SliderValue` (cast `/Game/Blueprints/BP_GameInstance` (`GameplayStatics.GetGameInstance`) :!pure true)) 1400.0)
    (`self.ResetPause`)
    (`/Engine/EditorBlueprintResources/StandardMacros.DoOnce` false :!label _label
      (:`Completed`
        (`self.StartBigScreen`)))
    (else
      (`/Engine/EditorBlueprintResources/StandardMacros.DoOnce` false :!label _label_2
        (:`Completed`
          (`self.SetPause`)
          (goto _label :!via `Reset`))))))

(event `ResetPause`
  (goto _label_2 :!via `Reset`))

(fn `UserConstructionScript`)