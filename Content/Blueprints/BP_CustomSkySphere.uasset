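; BP_CustomSkySphere is a sky sphere whose spin and sun height follow a slider value stored in BP_GameInstance.
; Each tick it yaws the sky mesh at a speed proportional to that value.
; Crossing a high threshold switches SunHeight between a raised and a lowered setting and refreshes the material.
; Two DoOnce gates reset each other, with ResetPause clearing one, so the refresh fires only on each change.
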(event `self.ReceiveBeginPlay`)

(event `self.ReceiveTick`
  (params (DeltaSeconds :type "Float (single-precision)"))
  (`SceneComponent.K2_AddWorldRotation` (`self.SkySphereMesh`) (`KismetMathLibrary.MakeRotator` 0.0 0.0 (* (* (/ (`/Game/Blueprints/BP_GameInstance.SliderValue` (cast `/Game/Blueprints/BP_GameInstance` (`GameplayStatics.GetGameInstance`) :!pure true)) 1500.0) -5.0) DeltaSeconds)) false false)
  (if (> (`/Game/Blueprints/BP_GameInstance.SliderValue` (cast `/Game/Blueprints/BP_GameInstance` (`GameplayStatics.GetGameInstance`) :!pure true)) 1400.0)
    (`self.ResetPause`)
    (`/Engine/EditorBlueprintResources/StandardMacros.DoOnce` false :!label _label
      (:`Completed`
        (set `self.Sun height` 0.6)
        (`self.RefreshMaterial`)))
    (else
      (`/Engine/EditorBlueprintResources/StandardMacros.DoOnce` false :!label _label_2
        (:`Completed`
          (set `self.Sun height` -0.9)
          (`self.RefreshMaterial`)
          (goto _label :!via `Reset`))))))

(event `ResetPause`
  (goto _label_2 :!via `Reset`))

(fn `UserConstructionScript`
  (`parent.UserConstructionScript`))